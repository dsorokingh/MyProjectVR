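; Plane actor that moves into place and plays a trailer video with sound once the column widget signals it is filled.
; On BeginPlay it casts the user widget on the referenced Column to ColumnWidget_Blueprint and binds to its Filled event.
; That event plays a timeline driving the actor's Z at fixed X.
; When the timeline finishes, MediaPlayer opens the trailer and the audio plays separately as a 2D sound.
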(event Custom|Filled_Event_0
  ;[1 1 1] Поднятие плоскости и запуск видео при нажатии на кнопку
  (bind _z (Timeline|Timeline_0 Play)
    (:Update
      (Transformation|SetActorLocation (Math|Vector|MakeVector 1.5e+02 0.0 _z) false false))
    (:Finished
      (Media|MediaPlayer|OpenSource (Variables|Default|GetMediaPlayer) "/Game/Video/bf4_trailer.bf4_trailer")
      (Audio|PlaySound2D "/Game/Video/bf4_trailer_audio.bf4_trailer_audio" 1.0 1.0 0.0 0 0))))

(event EventBeginPlay
  ;[1 1 1] Поднятие плоскости и запуск видео при нажатии на кнопку
  (bind _ascolumn_widget_blueprint (Utilities|Casting|CastToColumnWidget_Blueprint (UserInterface|GetUserWidgetObject (Variables|/Game/Blueprints/Column_Blueprint.Column_Blueprint_C|GetWidget (Variables|Default|GetColumn)))))
  (EventDispatchers|AssignFilled _ascolumn_widget_blueprint (delegate Custom|Filled_Event_0)))

(event Collision|EventActorBeginOverlap
  (params (OtherActor :type Actor%20Object%20Reference)))

(event EventTick
  (params (DeltaSeconds :type Float%20%28single-precision%29)))

(fn ConstructionScript)